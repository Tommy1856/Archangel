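; Exit portal actor for the Griffon boss fight, with a sphere, mesh and spark particles that start hidden.
; On BeginPlay it hides all three, casts its owner to GriffonBoss and re-shows only the sphere if that boss is not alive.
; The boss state is checked only once, and overlapping the sphere just prints a "Goodbye!" message, with no travel logic.
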(event `self.ReceiveBeginPlay`
  (bind _sphere (`self.Sphere`))
  (`|ExecutionSequence`
    (:`then_0`
      (`SceneComponent.SetVisibility` _sphere false false)
      (`SceneComponent.SetVisibility` (`self.StaticMesh`) false false)
      (`SceneComponent.SetVisibility` (`self.P_Sparks`) false false)
      (bind _asgriffon_boss (cast `/Game/Archangel/GriffionBoss/GriffonBoss` (`self.GetOwner`)))
      (if (not (`/Game/Archangel/GriffionBoss/GriffonBoss.Alive` _asgriffon_boss))
        (`SceneComponent.SetVisibility` _sphere true false)))))

(event `self.Sphere.OnComponentBeginOverlap`
  (params (OverlappedComponent :type "PrimitiveComponent Object Reference") (OtherActor :type "Actor Object Reference") (OtherComp :type "PrimitiveComponent Object Reference") (OtherBodyIndex :type Integer) (bFromSweep :type Boolean) (SweepResult :type "HitResult Structure (by ref)"))
  (`KismetSystemLibrary.PrintString` "Goodbye!"))

(fn `UserConstructionScript`)